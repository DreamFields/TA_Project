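; BP_CustomLoc2D is an FX Blueprint that moves its Niagara component along a spline once over MoveTime.
; Tick accumulates elapsed time in Alpha0 and maps it linearly to spline distance to set world location, with no further updates once MoveTime is exceeded.
; EnableStaticMeshRotate makes rotation follow the spline; otherwise it holds the spline's starting rotation.
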(event EventBeginPlay)

(event Collision|EventActorBeginOverlap
  (params (OtherActor :type Actor%20Object%20Reference)))

(event EventTick
  (params (DeltaSeconds :type Float%20%28single-precision%29))
  (bind _spline0 (Variables|Default|GetSpline0))
  (bind _output_get (Variables|Default|SetAlpha0 (+ (Variables|Default|GetAlpha0) DeltaSeconds)))
  (if (<= _output_get (Variables|Default|GetMoveTime))
    (Transformation|SetWorldLocation (Variables|Default|GetNiagara) (Spline|GetLocationatDistanceAlongSpline _spline0 (Math|Float|Lerp 0.0 (Spline|GetSplineLength _spline0) (/ (Variables|Default|GetAlpha0) (Variables|Default|GetMoveTime))) "World") false false)
    (if (Variables|Default|GetEnableStaticMeshRotate)
      (Transformation|SetWorldRotation (Variables|Default|GetNiagara) (Spline|GetRotationatDistanceAlongSpline _spline0 (Math|Float|Lerp 0.0 (Spline|GetSplineLength _spline0) (/ (Variables|Default|GetAlpha0) (Variables|Default|GetMoveTime))) "World") false false)
      (else
        (Transformation|SetWorldRotation (Variables|Default|GetNiagara) (Spline|GetRotationatDistanceAlongSpline (Variables|Default|GetSpline0) 0.0 "World") false false)))))

(fn ConstructionScript)