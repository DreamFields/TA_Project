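; BP_BoidFish is an actor that drives a Niagara boid fish effect, feeding it the player's position and movement state.
; The construction script passes grid resolution and size to the FXFish system.
; Each tick it sets the player's location and flags movement when the player is beyond a small distance threshold from the stored previous location, which updates only when that threshold is exceeded.
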(event EventBeginPlay)

(event Collision|EventActorBeginOverlap
  (params (OtherActor :type Actor%20Object%20Reference)))

(event EventTick
  (params (DeltaSeconds :type Float%20%28single-precision%29))
  (bind _returnvalue (Game|GetPlayerCharacter 0))
  (bind _returnvalue_2 (Transformation|GetActorLocation _returnvalue))
  (Niagara|SetNiagaraVariable(Vector3) (Variables|Default|GetFX_Fish) "PlayerLocation" _returnvalue_2)
  (Class|NiagaraComponent|SetVariableBool (Variables|Default|GetFX_Fish) "IsPlayerMoving" (> (Math|Vector|Distance(Vector) (Variables|Default|GetPreLocation) _returnvalue_2) 0.5))
  (if (> (Math|Vector|Distance(Vector) (Variables|Default|GetPreLocation) _returnvalue_2) 0.5)
    (Variables|Default|SetPreLocation _returnvalue_2)))

(fn ConstructionScript
  (Niagara|SetNiagaraVariable(Vector3) (Variables|Default|GetFX_Fish) "GridResolution" (Variables|Default|GetGridResolution))
  (Niagara|SetNiagaraVariable(Vector3) (Variables|Default|GetFX_Fish) "GridSize" (Variables|Default|GetGridSize)))