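; Niagara boid fish school actor that feeds player presence and movement into its FXMultiFish simulation.
; The construction script pushes grid, mesh, material and color array settings to Niagara and sizes the trigger box from GenerateSize.
; Box overlaps, unfiltered by actor, toggle IsHavePlayer and print debug strings.
; While it is set, Tick sends the player's location and a moving flag derived from a small distance threshold.
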(event OnComponentBeginOverlap(BoxCollision)
  (params (OverlappedComponent :type Primitive%20Component%20Object%20Reference) (OtherActor :type Actor%20Object%20Reference) (OtherComp :type Primitive%20Component%20Object%20Reference) (OtherBodyIndex :type Integer) (bFromSweep :type Boolean) (SweepResult :type Hit%20Result%20Structure%20%28by%20ref%29))
  (Variables|Default|SetIsHavePlayer true)
  (Class|NiagaraComponent|SetVariableBool (Variables|Default|GetFX_MultiFish) "IsHavePlayer" true)
  (Development|PrintString "in"))

(event OnComponentEndOverlap(BoxCollision)
  (params (OverlappedComponent :type Primitive%20Component%20Object%20Reference) (OtherActor :type Actor%20Object%20Reference) (OtherComp :type Primitive%20Component%20Object%20Reference) (OtherBodyIndex :type Integer))
  (Variables|Default|SetIsHavePlayer false)
  (Class|NiagaraComponent|SetVariableBool (Variables|Default|GetFX_MultiFish) "IsHavePlayer" false)
  (Development|PrintString "out"))

(event EventBeginPlay)

(event Collision|EventActorBeginOverlap
  (params (OtherActor :type Actor%20Object%20Reference)))

(event EventTick
  (params (DeltaSeconds :type Float%20%28single-precision%29))
  (bind _returnvalue (Game|GetPlayerCharacter 0))
  (bind _returnvalue_2 (Transformation|GetActorLocation _returnvalue))
  (if (Variables|Default|GetIsHavePlayer)
    (Niagara|SetNiagaraVariable(Vector3) (Variables|Default|GetFX_MultiFish) "PlayerLocation" _returnvalue_2)
    (Class|NiagaraComponent|SetVariableBool (Variables|Default|GetFX_MultiFish) "IsPlayerMoving" (> (Math|Vector|Distance(Vector) (Variables|Default|GetPreLocation) _returnvalue_2) 0.5))
    (if (> (Math|Vector|Distance(Vector) (Variables|Default|GetPreLocation) _returnvalue_2) 0.5)
      (Variables|Default|SetPreLocation _returnvalue_2))
    (else
      (Class|NiagaraComponent|SetVariableBool (Variables|Default|GetFX_MultiFish) "IsPlayerMoving" false))))

(fn ConstructionScript
  (bind _fx_multifish (Variables|Default|GetFX_MultiFish))
  (Niagara|SetNiagaraVariable(Vector3) _fx_multifish "GridResolution" (Variables|Default|GetGridResolution))
  (Niagara|SetNiagaraVariable(Vector3) _fx_multifish "GridSize" (Variables|Default|GetGenerateSize))
  (Class|NiagaraComponent|SetVariableStaticMesh _fx_multifish "SMHuman" (Variables|Default|GetStaticMeshTest))
  (Class|NiagaraComponent|SetVariableMaterial _fx_multifish "Material Interface" (Variables|Default|GetMaterialInterfaceTest))
  (Class|NiagaraDataInterfaceArrayFunctionLibrary|SetNiagaraArrayColor _fx_multifish "Color Array" (Variables|Default|GetColors))
  (Components|Box|SetBoxExtent (Variables|Default|GetBoxCollision) (Variables|Default|GetGenerateSize) true))