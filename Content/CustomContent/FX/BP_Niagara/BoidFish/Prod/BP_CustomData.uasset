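; Actor that drives a Niagara boid fish effect reacting to the player inside a box volume.
; Construction passes meshes and cumulative count arrays for mesh and weighted color selection to Niagara, sizing box and grid from GenerateSize.
; Tick deactivates the effect when the player is distant, reactivates it nearby, and pauses it when behind the camera with the box empty.
; Box overlaps toggle player presence, enabling player location and movement updates to Niagara.
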(event OnComponentBeginOverlap(Box)
  (params (OverlappedComponent :type Primitive%20Component%20Object%20Reference) (OtherActor :type Actor%20Object%20Reference) (OtherComp :type Primitive%20Component%20Object%20Reference) (OtherBodyIndex :type Integer) (bFromSweep :type Boolean) (SweepResult :type Hit%20Result%20Structure%20%28by%20ref%29))
  ;[1 1 1] 判断玩家是否进入包围盒
  (Variables|Default|SetIsHavePlayer true)
  (Class|NiagaraComponent|SetVariableBool (Variables|Default|GetFX_Custom) "IsHavePlayer" true)
  (Development|PrintString "in"))

(event OnComponentEndOverlap(Box)
  (params (OverlappedComponent :type Primitive%20Component%20Object%20Reference) (OtherActor :type Actor%20Object%20Reference) (OtherComp :type Primitive%20Component%20Object%20Reference) (OtherBodyIndex :type Integer))
  ;[1 1 1] 判断玩家是否进入包围盒
  (Variables|Default|SetIsHavePlayer false)
  (Class|NiagaraComponent|SetVariableBool (Variables|Default|GetFX_Custom) "IsHavePlayer" false)
  (Development|PrintString "out"))

(event EventBeginPlay)

(event Collision|EventActorBeginOverlap
  (params (OtherActor :type Actor%20Object%20Reference))
  ;[1 1 1] 测试代码
)

(event EventTick
  (params (DeltaSeconds :type Float%20%28single-precision%29))
  (bind _returnvalue (Game|GetPlayerCameraManager 0))
  (bind _returnvalue_2 (Game|Player|GetPlayerPawn 0))
  (bind _fx_custom (Variables|Default|GetFX_Custom))
  (bind _fx_custom_2 (Variables|Default|GetFX_Custom))
  (bind _returnvalue_3 (Transformation|GetWorldLocation _fx_custom))
  (bind _returnvalue_4 (Transformation|GetActorLocation _returnvalue_2))
  ;[1 1 1] 判断粒子系统是否应该注销
  (if (> (Math|Vector|Distance(Vector) (Transformation|GetActorLocation (Game|Player|GetPlayerPawn 0)) _returnvalue_3) 5e+03)
    (Class|FXSystemComponent|DeactivateImmediate (Variables|Default|GetFX_Custom))
    (else
      ;;[1 0.05092 0.03103] 当粒子数量减为0时，系统会自动Deactivate，从而Active=false，于是重新激活系统
      (if (Components|Activation|IsActive (Variables|Default|GetFX_Custom))
        _
        (else
          (Class|FXSystemComponent|ActivateSystem (Variables|Default|GetFX_Custom) false)))
      ;[1 1 1] 判断粒子系统是否应该运行模拟
      (Class|NiagaraComponent|SetPaused (Variables|Default|GetFX_Custom) (and (< (Math|Vector|DotProduct (Math|Vector|Normalize (Transformation|GetActorForwardVector _returnvalue)) (Math|Vector|Normalize (- _returnvalue_3 (Transformation|GetActorLocation _returnvalue)))) 0.0) (not (Variables|Default|GetIsHavePlayer))))
      ;[1 1 1] 判断玩家是否静止
      (if (Variables|Default|GetIsHavePlayer)
        (Niagara|SetNiagaraVariable(Vector3) _fx_custom_2 "PlayerLocation" _returnvalue_4)
        (Class|NiagaraComponent|SetVariableBool _fx_custom_2 "IsPlayerMoving" (> (Math|Vector|Distance(Vector) (Variables|Default|GetPreLocation) _returnvalue_4) 0.5))
        (if (> (Math|Vector|Distance(Vector) (Variables|Default|GetPreLocation) _returnvalue_4) 0.5)
          (Variables|Default|SetPreLocation _returnvalue_4))
        (else
          (Class|NiagaraComponent|SetVariableBool (Variables|Default|GetFX_Custom) "IsPlayerMoving" false))))))

(fn ConstructionScript
  (bind _fx_custom (Variables|Default|GetFX_Custom))
  (for (_array_element _array_index) (Variables|Default|GetMeshArray)
    ;[0.5943 0.6746 1] 设置不同的Mesh
    (Class|NiagaraComponent|SetVariableStaticMesh (Variables|Default|GetFX_Custom) (|SetVaribleName_2_2_2 _array_index) (.Mesh (Utilities|Struct|BreakMeshStruct _array_element)))
    ;[0.1244 1 0.9702] 设置该Mesh所有颜色的总权重
    (Variables|Default|SetTotalWeight 0.0)
    (for _array_element_2 (.ColorWeight (Utilities|Struct|BreakMeshStruct _array_element))
      (Variables|Default|SetTotalWeight (+ (Variables|Default|GetTotalWeight) (.Weight (Utilities|Struct|BreakColorWeight _array_element_2)))))
    ;[1 1 1] 计算粒子的Color的Array，索引对应粒子的执行索引
    (for _array_element_3 (.ColorWeight (Utilities|Struct|BreakMeshStruct _array_element))
      (bind _output_get (Variables|Default|SetColorNum (+ (|SetLoopNum_2_2_2 (.Weight (Utilities|Struct|BreakColorWeight _array_element_3)) (.Number (Utilities|Struct|BreakMeshStruct _array_element))) (Variables|Default|GetColorNum))))
      (Utilities|Array|Add (Variables|Default|GetColorNumArray) _output_get)
      (Utilities|Array|Add (Variables|Default|GetColorArray) (Math|Conversions|ToLinearColor(Color) (.Color (Utilities|Struct|BreakColorWeight _array_element_3)))))
    ;[1 1 1] 计算总粒子数
    (bind _output_get_2 (Variables|Default|SetTotalNum (+ (Variables|Default|GetTotalNum) (.Number (Utilities|Struct|BreakMeshStruct _array_element)))))
    (Utilities|Array|Add (Variables|Default|GetMeshNumArray) _output_get_2))
  ;[1 1 1] 传递给粒子系统
  (Class|NiagaraDataInterfaceArrayFunctionLibrary|SetNiagaraArrayInt32 _fx_custom "MeshNumArray" (Variables|Default|GetMeshNumArray))
  (Class|NiagaraComponent|SetVariableInt _fx_custom "TotalNum" (Variables|Default|GetTotalNum))
  (Class|NiagaraDataInterfaceArrayFunctionLibrary|SetNiagaraArrayColor _fx_custom "ColorArray" (Variables|Default|GetColorArray))
  (Class|NiagaraDataInterfaceArrayFunctionLibrary|SetNiagaraArrayInt32 _fx_custom "ColorNumArray" (Variables|Default|GetColorNumArray))
  (Niagara|SetNiagaraVariable(Vector3) _fx_custom "GridSize" (* (Variables|Default|GetGenerateSize) "2.000000,2.000000,2.000000"))
  (Components|Box|SetBoxExtent (Variables|Default|GetBox) (Variables|Default|GetGenerateSize) true))