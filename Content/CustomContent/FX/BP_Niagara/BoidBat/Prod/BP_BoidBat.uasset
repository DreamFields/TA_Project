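; Bat swarm FX actor that moves a Niagara system along up to three splines through timed states: boid simulation, tornado or static mesh.
; The construction script pauses Niagara and turns each StateSet entry's wait and move durations into cumulative times.
; While visible, Tick finds the current state, sets its mode, snaps the next spline's start to the current end, then waits or moves.
; Older single-transform logic remains unwired.
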(event EventTick
  (params (DeltaSeconds :type Float%20%28single-precision%29))
  (bind _timesat (Variables|Default|GetTimeSAT))
  (bind _niagara (Variables|Default|GetNiagara))
  (if (not (Variables|Rendering|GetbHidden))
    (bind _output_get (Variables|Default|SetTempTime (+ DeltaSeconds (Variables|Default|GetTempTime))))
    (bind _curindex (CallFunction|GetIndex _output_get))
    (bind _output_get_2 (Variables|Default|SetCurIndex _curindex))
    ;[1 1 1] 把下一个样条线的第0个点设置为现在样条线的最后一个点
    (if (!= _output_get_2 -1)
      (if (< (+ _output_get_2 1) (Utilities|Array|Length (Variables|Default|GetStateSet)))
        (bind _newparam (CallFunction|GetSpline (Variables|Default|GetCurIndex)))
        (bind _newparam_2 (CallFunction|GetSpline (+ _output_get_2 1)))
        (Spline|SetLocationatSplinePoint _newparam_2 0 (Spline|GetLocationatDistanceAlongSpline _newparam (Spline|GetSplineLength _newparam) "World") "World" true)
        (Variables|Private|SetNiagaraRotation (Transformation|GetWorldRotation (Variables|Default|GetNiagara))))
      (Class|NiagaraComponent|SetVariableBool _niagara "EnableBoidSimulation" (== (Math|Conversions|ToInteger(Byte) (.Mode (Utilities|Struct|BreakStateSet (Utilities|Array|Get(acopy) (Variables|Default|GetStateSet) (Variables|Default|GetCurIndex))))) 0))
      (Class|NiagaraComponent|SetVariableBool _niagara "EnableTornado" (== (Math|Conversions|ToInteger(Byte) (.Mode (Utilities|Struct|BreakStateSet (Utilities|Array|Get(acopy) (Variables|Default|GetStateSet) (Variables|Default|GetCurIndex))))) 1))
      (Class|NiagaraComponent|SetVariableBool _niagara "EnableStaticMesh" (== (Math|Conversions|ToInteger(Byte) (.Mode (Utilities|Struct|BreakStateSet (Utilities|Array|Get(acopy) (Variables|Default|GetStateSet) (Variables|Default|GetCurIndex))))) 2))
      (if (== (Math|Conversions|ToInteger(Byte) (.Mode (Utilities|Struct|BreakStateSet (Utilities|Array|Get(acopy) (Variables|Default|GetStateSet) (Variables|Default|GetCurIndex))))) 2)
        (Class|NiagaraComponent|SetVariableStaticMesh (Variables|Default|GetNiagara) "StaticMesh" (.StaticMesh (Utilities|Struct|BreakStateSet (Utilities|Array|Get(acopy) (Variables|Default|GetStateSet) (Variables|Default|GetCurIndex))))))
      (if (<= (Variables|Default|GetTempTime) (Utilities|Array|Get(acopy) _timesat (* (Variables|Default|GetCurIndex) 2)))
        ;[0.4214 0.8695 1] 设置粒子系统的旋转方向为切线方向 缓慢过渡
        (bind _newparam_3 (CallFunction|GetSpline (Variables|Default|GetCurIndex)))
        (if (== (Variables|Default|GetCurIndex) 0)
          (Variables|Default|SetTempAlpha (/ (Variables|Default|GetTempTime) (.StartWait (Utilities|Struct|BreakStateSet (Utilities|Array|Get(acopy) (Variables|Default|GetStateSet) (Variables|Default|GetCurIndex))))))
          (else
            (Variables|Default|SetTempAlpha (/ (- (Variables|Default|GetTempTime) (Utilities|Array|Get(acopy) (Variables|Default|GetTimeSAT) (- (* (Variables|Default|GetCurIndex) 2) 1))) 0.0))))
        (switch int (Math|Conversions|ToInteger(Byte) (.Mode (Utilities|Struct|BreakStateSet (Utilities|Array|Get(acopy) (Variables|Default|GetStateSet) (Variables|Default|GetCurIndex)))))
          (:2
            (Transformation|SetWorldRotation (Variables|Default|GetNiagara) (Math|Rotator|Lerp(Rotator) (Variables|Private|GetNiagaraRotation) (Spline|GetRotationatDistanceAlongSpline _newparam_3 0.0 "World") 0.0 true) false false)))
        (elif (<= (Variables|Default|GetTempTime) (Utilities|Array|Get(acopy) _timesat (+ (* (Variables|Default|GetCurIndex) 2) 1)))
          (bind _newparam_4 (CallFunction|GetSpline (Variables|Default|GetCurIndex)))
          (Transformation|SetWorldLocation (Variables|Default|GetNiagara) (Spline|GetLocationatDistanceAlongSpline _newparam_4 (Math|Float|Lerp 0.0 (Spline|GetSplineLength _newparam_4) (/ (- (Variables|Default|GetTempTime) (Utilities|Array|Get(acopy) _timesat (* (Variables|Default|GetCurIndex) 2))) (- (Utilities|Array|Get(acopy) _timesat (+ (* (Variables|Default|GetCurIndex) 2) 1)) (Utilities|Array|Get(acopy) _timesat (* (Variables|Default|GetCurIndex) 2))))) "World") false false))))))

(fn ConstructionScript
  (bind _niagara (Variables|Default|GetNiagara))
  (bind _timesat (Variables|Default|GetTimeSAT))
  (Class|NiagaraComponent|SetPaused _niagara true)
  (Class|NiagaraComponent|SetVariableBool _niagara "EnableBoidSimulation" true)
  (Class|NiagaraComponent|SetVariableBool _niagara "EnableTornado" false)
  (Class|NiagaraComponent|SetVariableBool _niagara "EnableStaticMesh" false)
  (for _array_element (Variables|Default|GetStateSet)
    (Utilities|Array|Add _timesat (+ (.StartWait (Utilities|Struct|BreakStateSet _array_element)) (Variables|Default|GetTempTime)))
    (Utilities|Array|Add _timesat (+ (+ (.StartWait (Utilities|Struct|BreakStateSet _array_element)) (Variables|Default|GetTempTime)) (.MoveTime (Utilities|Struct|BreakStateSet _array_element))))
    (Variables|Default|SetTempTime (+ (+ (.StartWait (Utilities|Struct|BreakStateSet _array_element)) (Variables|Default|GetTempTime)) (.MoveTime (Utilities|Struct|BreakStateSet _array_element))))
    (Development|PrintString "Hello"))
  (Variables|Default|SetTempTime 0.0))

(fn GetSpline
  (params (Index :type Integer))
  (if (== 0 Index)
    (return (Variables|Default|GetSpline0))
    (elif (== 1 Index)
      (return (Variables|Default|GetSpline1))
      (else
        (return (Variables|Default|GetSpline2))))))

(fn GetIndex
  (params (TempTime :type Float%20%28double-precision%29))
  (for _index (range 0 (- (Utilities|Array|Length (Variables|Default|GetStateSet)) 1))
    (if (<= TempTime (Utilities|Array|Get(acopy) (Variables|Default|GetTimeSAT) (+ (* _index 2) 1)))
      (return _index)))
  (return -1))