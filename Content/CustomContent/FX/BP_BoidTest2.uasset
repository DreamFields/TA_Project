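; BP_BoidTest2 is a test actor that makes an FX system, likely boids by its name, react to the player.
; The construction script sizes the trigger box from GenerateSize and sets the effect's GridSize to double that.
; Box overlaps toggle IsHavePlayer; while it is true, Tick feeds the effect player location and a distance-based moving flag.
; Distance and view-direction culling logic exists but is unconnected.
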(event OnComponentBeginOverlap(Box)
  (params (OverlappedComponent :type Primitive%20Component%20Object%20Reference) (OtherActor :type Actor%20Object%20Reference) (OtherComp :type Primitive%20Component%20Object%20Reference) (OtherBodyIndex :type Integer) (bFromSweep :type Boolean) (SweepResult :type Hit%20Result%20Structure%20%28by%20ref%29))
  ;[1 1 1] 判断玩家是否进入包围盒
  (Variables|Default|SetIsHavePlayer true)
  (Class|NiagaraComponent|SetVariableBool (Variables|Default|GetFX_Custom) "IsHavePlayer" true)
  (Development|PrintString "in"))

(event OnComponentEndOverlap(Box)
  (params (OverlappedComponent :type Primitive%20Component%20Object%20Reference) (OtherActor :type Actor%20Object%20Reference) (OtherComp :type Primitive%20Component%20Object%20Reference) (OtherBodyIndex :type Integer))
  ;[1 1 1] 判断玩家是否进入包围盒
  (Variables|Default|SetIsHavePlayer false)
  (Class|NiagaraComponent|SetVariableBool (Variables|Default|GetFX_Custom) "IsHavePlayer" false)
  (Development|PrintString "out"))

(event EventBeginPlay)

(event Collision|EventActorBeginOverlap
  (params (OtherActor :type Actor%20Object%20Reference)))

(event EventTick
  (params (DeltaSeconds :type Float%20%28single-precision%29))
  (bind _returnvalue (Game|Player|GetPlayerPawn 0))
  (bind _fx_custom (Variables|Default|GetFX_Custom))
  (bind _returnvalue_2 (Transformation|GetActorLocation _returnvalue))
  ;[1 1 1] 判断玩家是否静止
  (if (Variables|Default|GetIsHavePlayer)
    (Niagara|SetNiagaraVariable(Vector3) _fx_custom "PlayerLocation" _returnvalue_2)
    (Class|NiagaraComponent|SetVariableBool _fx_custom "IsPlayerMoving" (> (Math|Vector|Distance(Vector) (Variables|Default|GetPreLocation) _returnvalue_2) 0.5))
    (if (> (Math|Vector|Distance(Vector) (Variables|Default|GetPreLocation) _returnvalue_2) 0.5)
      (Variables|Default|SetPreLocation _returnvalue_2))
    (else
      (Class|NiagaraComponent|SetVariableBool (Variables|Default|GetFX_Custom) "IsPlayerMoving" false))))

(fn ConstructionScript
  (Niagara|SetNiagaraVariable(Vector3) (Variables|Default|GetFX_Custom) "GridSize" (* (Variables|Default|GetGenerateSize) "2.000000,2.000000,2.000000"))
  (Components|Box|SetBoxExtent (Variables|Default|GetBox) (Variables|Default|GetGenerateSize) true))